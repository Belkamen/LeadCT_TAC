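; Projectile actor that deals damage to whatever it hits.
; On BeginPlay its Box component ignores the instigator while moving, and the actor destroys itself after a short lifetime.
; On a hit it applies fixed damage to a valid actor with the instigator as damage causer, plays a 2D hit sound, then destroys itself.
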(event `self.ReceiveBeginPlay`
  (`PrimitiveComponent.IgnoreActorWhenMoving` (`self.Box`) (`self.GetInstigator`) true)
  (`KismetSystemLibrary.Delay` 3.0)
  (`self.K2_DestroyActor`))

(event `self.ReceiveHit`
  (params (MyComp :type "PrimitiveComponent Object Reference") (Other :type "Actor Object Reference") (OtherComp :type "PrimitiveComponent Object Reference") (bSelfMoved :type Boolean) (HitLocation :type "Vector Structure") (HitNormal :type "Vector Structure") (NormalImpulse :type "Vector Structure") (Hit :type "HitResult Structure (by ref)"))
  (`/Engine/EditorBlueprintResources/StandardMacros.IsValid` Other
    (:`Is Valid`
      (`GameplayStatics.ApplyDamage` Other 1.0 null (`self.GetInstigator`))
      (`GameplayStatics.SpawnSound2D` "/Game/Assets/SFX/hit1__2__Cue.hit1__2__Cue" 1.0 1.0 0.0 null))
    (:`Is Not Valid`
      _))
  (`self.K2_DestroyActor`))

(fn `UserConstructionScript`)