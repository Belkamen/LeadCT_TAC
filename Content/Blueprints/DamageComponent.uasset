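; Actor component that gives its owner health, reacts to any damage it takes and destroys it when health runs out.
; Each hit spawns a tinted Niagara impact and briefly flashes the owner's Paper2D flipbook red, if it has one.
; With HaveBlood set, it also spawns a blood emitter aimed at the damage causer, whose particle collisions leave randomly sized and rotated blood decals.
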(event `self.ReceiveBeginPlay`
  (add `Actor.OnTakeAnyDamage` (`self.GetOwner`) (delegate `Damage`)))

(event `Damage`
  (params (DamagedActor :type "Actor Object Reference") (Damage :type "Float (double-precision)") (DamageType :type "DamageType Object Reference") (InstigatedBy :type "Controller Object Reference") (DamageCauser :type "Actor Object Reference"))
  (set `self.Damager` DamageCauser)
  (bind _output_get (set `self.Health` (- (`self.Health`) Damage)))
  (if (<= _output_get 0.0)
    (`self.VisualEffects`)
    (`Actor.K2_DestroyActor` (`self.GetOwner`))
    (else
      (`self.VisualEffects`))))

(event `VisualEffects`
  (bind _returnvalue_location (`KismetMathLibrary.BreakTransform` (`Actor.GetTransform` (`self.GetOwner`))))
  (bind _returnvalue (`Actor.GetComponentByClass` (`self.GetOwner`) "/Script/Paper2D.PaperFlipbookComponent"))
  (if (`self.bHaveBlood?`)
    (`self.BloodMechanic`))
  (bind _returnvalue_2 (`NiagaraFunctionLibrary.SpawnSystemAtLocation` "/Game/Assets/FX/Niagara_FX/FX_hit_impact.FX_hit_impact" _returnvalue_location))
  (`FXSystemComponent.SetColorParameter` _returnvalue_2 "Color" (struct :`R` 15.0 :`G` 5.0 :`B` 0.364242 :`A` 1.0))
  (`FXSystemComponent.SetFloatParameter` _returnvalue_2 "Scale" 3.0)
  (`/Engine/EditorBlueprintResources/StandardMacros.IsValid` _returnvalue
    (:`Is Valid`
      (`PaperFlipbookComponent.SetSpriteColor` _returnvalue (struct :`R` 150.0 :`A` 1.0))
      (`KismetSystemLibrary.Delay` (`KismetMathLibrary.RandomFloatInRange` 0.1 0.3))
      (`PaperFlipbookComponent.SetSpriteColor` _returnvalue (struct :`R` 1.0 :`G` 1.0 :`B` 1.0 :`A` 1.0)))))

(fn `BloodMechanic`
  (bind _returnvalue (`Actor.K2_GetActorLocation` (`self.GetOwner`)))
  (bind _returnvalue_2 (`GameplayStatics.SpawnEmitterAtLocation` "/Game/Assets/FX/BloodSplash.BloodSplash" _returnvalue (`KismetMathLibrary.FindLookAtRotation` _returnvalue (`Actor.K2_GetActorLocation` (`self.Damager`)))))
  (add `ParticleSystemComponent.OnParticleCollide` _returnvalue_2 (`|CreateDelegate` :!event `DamageComponent_AutoGenFunc`)))

(fn `DamageComponent_AutoGenFunc`
  (params (EventName :type Name) (EmitterTime :type "Float (double-precision)") (ParticleTime :type Integer) (Location :type "Vector Structure") (Velocity :type "Vector Structure") (Direction :type "Vector Structure") (Normal :type "Vector Structure") (BoneName :type Name) (PhysMat :type "PhysicalMaterial Object Reference"))
  (bind _returnvalue (`KismetMathLibrary.RandomFloatInRange` 64.0 128.0))
  (`GameplayStatics.SpawnDecalAtLocation` "/Game/Assets/Materials/Blood/MI_D_Blood_01.MI_D_Blood_01" (`KismetMathLibrary.MakeVector` 50.0 _returnvalue _returnvalue) Location (`KismetMathLibrary.MakeRotator` (.roll (`KismetMathLibrary.Conv_VectorToRotator` Normal)) (.pitch (`KismetMathLibrary.Conv_VectorToRotator` Normal)) (`KismetMathLibrary.RandomFloatInRange` -90.0 90.0)) 150.0)
  (return))